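; Player character Blueprint that maps ACF input actions to movement, jumping, crouching, walking and sprinting.
; Move input feeds LocomotionComp, while stance and gait changes go to CTCmptLocomotion.
; Crouch callbacks switch between Crouch and Jog, walk input toggles Walk/Jog, and CanSprint allows sprint only in Jog.
; The T key toggles strafing and forward-facing rotation; a second forward-input handler checks a threshold but does nothing.
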(event EventBeginPlay
  (|CallParentFunction) ; This node is disabled and will not be called.\nDrag off pins to build functionality.
)

(event Collision|EventActorBeginOverlap
  (params (OtherActor :type Actor%20Object%20Reference))
  (|CallParentFunction OtherActor) ; This node is disabled and will not be called.\nDrag off pins to build functionality.
)

(event EventTick
  (params (DeltaSeconds :type Float%20%28single-precision%29)))

(event Input|EnhancedActionEvents|EnhancedInputActionACFCrouchInput
  (params (ActionValue :type Boolean) (ElapsedSeconds :type Float%20%28double-precision%29) (TriggeredSeconds :type Float%20%28double-precision%29) (InputAction :type Input%20Action%20Object%20Reference :default "/AscentCombatFramework/Input/ACFCrouchInput.ACFCrouchInput"))
  ;[1 1 1] Crouch
  (if (Variables|Default|GetbIsCrouched)
    (Character|UnCrouch)
    (else
      (Character|Crouch))))

(event Input|EnhancedActionEvents|EnhancedInputActionACFMoveRightInput
  (params (ActionValue :type Float%20%28double-precision%29) (ElapsedSeconds :type Float%20%28double-precision%29) (TriggeredSeconds :type Float%20%28double-precision%29) (InputAction :type Input%20Action%20Object%20Reference :default "/AscentCombatFramework/Input/ACFMoveRightInput.ACFMoveRightInput"))
  ;[1 1 1] Move, Jump
  (Class|ACFCharacterMovementComponent|MoveRight (Variables|Default|GetLocomotionComp) ActionValue))

(event Input|EnhancedActionEvents|EnhancedInputActionACFJumpInput
  (params (ActionValue :type Boolean) (ElapsedSeconds :type Float%20%28double-precision%29) (TriggeredSeconds :type Float%20%28double-precision%29) (InputAction :type Input%20Action%20Object%20Reference :default "/AscentCombatFramework/Input/ACFJumpInput.ACFJumpInput"))
  ;[1 1 1] Move, Jump
  (Character|Jump))

(event Input|EnhancedActionEvents|EnhancedInputActionACFMoveForwardInput
  (params (ActionValue :type Float%20%28double-precision%29) (ElapsedSeconds :type Float%20%28double-precision%29) (TriggeredSeconds :type Float%20%28double-precision%29) (InputAction :type Input%20Action%20Object%20Reference :default "/AscentCombatFramework/Input/ACFMoveForwardInput.ACFMoveForwardInput"))
  ;[1 1 1] Walk
  (if (< ActionValue 0.4)
    _))

(event Input|EnhancedActionEvents|EnhancedInputActionACFSprintInput
  (params (ActionValue :type Boolean) (ElapsedSeconds :type Float%20%28double-precision%29) (TriggeredSeconds :type Float%20%28double-precision%29) (InputAction :type Input%20Action%20Object%20Reference :default "/AscentCombatFramework/Input/ACFSprintInput.ACFSprintInput"))
  (bind _ct_cmpt_locomotion (Variables|Default|GetCT_Cmpt_Locomotion))
  ;[1 1 1] Sprint
  (:Started
    (if (CallFunction|CanSprint)
      (Default|SetSprint _ct_cmpt_locomotion true)))
  (:Completed
    (Default|SetSprint _ct_cmpt_locomotion false)))

(event Input|EnhancedActionEvents|EnhancedInputActionACFWalk_AJ
  (params (ActionValue :type Boolean) (ElapsedSeconds :type Float%20%28double-precision%29) (TriggeredSeconds :type Float%20%28double-precision%29) (InputAction :type Input%20Action%20Object%20Reference :default "/AscentCombatFramework/Input/ACFWalk_AJ.ACFWalk_AJ"))
  (bind _ct_cmpt_locomotion (Variables|Default|GetCT_Cmpt_Locomotion))
  ;[1 1 1] Walk
  (switch Utilities|FlowControl|Switch|SwitchonEnum_MovementType (Default|GetMovementType (Variables|Default|GetCT_Cmpt_Locomotion))
    (:NewEnumerator0
      (Default|SetMovementType _ct_cmpt_locomotion "NewEnumerator1"))
    (:NewEnumerator1
      (Default|SetMovementType _ct_cmpt_locomotion "NewEnumerator0")
      (Default|SetSprint (Variables|Default|GetCT_Cmpt_Locomotion) false))))

(event Input|EnhancedActionEvents|EnhancedInputActionACFMoveForwardInput
  (params (ActionValue :type Float%20%28double-precision%29) (ElapsedSeconds :type Float%20%28double-precision%29) (TriggeredSeconds :type Float%20%28double-precision%29) (InputAction :type Input%20Action%20Object%20Reference :default "/AscentCombatFramework/Input/ACFMoveForwardInput.ACFMoveForwardInput"))
  ;[1 1 1] Move, Jump
  (Class|ACFCharacterMovementComponent|MoveForward (Variables|Default|GetLocomotionComp) ActionValue))

(event EventOnStartCrouch
  (params (HalfHeightAdjust :type Float%20%28single-precision%29) (ScaledHalfHeightAdjust :type Float%20%28single-precision%29))
  ;[1 1 1] Crouch
  (Default|SetMovementType (Variables|Default|GetCT_Cmpt_Locomotion) "NewEnumerator3")
  (Default|SetSprint (Variables|Default|GetCT_Cmpt_Locomotion) false))

(event EventOnEndCrouch
  (params (HalfHeightAdjust :type Float%20%28single-precision%29) (ScaledHalfHeightAdjust :type Float%20%28single-precision%29))
  ;[1 1 1] Crouch
  (Default|SetMovementType (Variables|Default|GetCT_Cmpt_Locomotion) "NewEnumerator1"))

(event Input|KeyboardEvents|T
  (params (Key :type Key%20Structure :default "None"))
  (bind _ct_cmpt_locomotion (Variables|Default|GetCT_Cmpt_Locomotion))
  ;[1 1 1] Rotation mode
  (:Pressed
    (switch Utilities|FlowControl|Switch|SwitchonEnum_RotationMode (Default|GetRotationMode (Variables|Default|GetCT_Cmpt_Locomotion))
      (:NewEnumerator0
        (Default|SetRotationMode _ct_cmpt_locomotion "NewEnumerator1"))
      (:NewEnumerator1
        (Default|SetRotationMode _ct_cmpt_locomotion "NewEnumerator0")))))

(fn ConstructionScript
  (|CallParentFunction))

(fn CanSprint
  (return (Default|IsMovementType (Variables|Default|GetCT_Cmpt_Locomotion) "NewEnumerator1")))