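; BP_PlayerController_AJ is a player controller that sets up Enhanced Input and handles turn and look-up camera input.
; On BeginPlay it calls its parent and adds a mapping context to the local player's input subsystem.
; Turn and look-up actions feed yaw and pitch, each scaled by frame delta time, a per-axis sensitivity and a base turn rate.
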(event Input|EnhancedActionEvents|EnhancedInputActionACFTurnInput
  (params (ActionValue :type Float%20%28double-precision%29) (ElapsedSeconds :type Float%20%28double-precision%29) (TriggeredSeconds :type Float%20%28double-precision%29) (InputAction :type Input%20Action%20Object%20Reference :default "/AscentCombatFramework/Input/ACFTurnInput.ACFTurnInput"))
  (Class|PlayerController|AddYawInput (* ActionValue (Utilities|Time|GetWorldDeltaSeconds) (Class|ACFPlayerController|GetXSensitivity) (Variables|Default|GetBaseTurnrate))))

(event Input|EnhancedActionEvents|EnhancedInputActionACFLookUpInput
  (params (ActionValue :type Float%20%28double-precision%29) (ElapsedSeconds :type Float%20%28double-precision%29) (TriggeredSeconds :type Float%20%28double-precision%29) (InputAction :type Input%20Action%20Object%20Reference :default "/AscentCombatFramework/Input/ACFLookUpInput.ACFLookUpInput"))
  (Class|PlayerController|AddPitchInput (* ActionValue (Utilities|Time|GetWorldDeltaSeconds) (Class|ACFPlayerController|GetYSensitivity) (Variables|Default|GetBaseTurnrate))))

(event EventBeginPlay
  (bind _returnvalue (PlayerController|LocalPlayerSubsystems|GetEnhancedInputLocalPlayerSubsystem))
  (|CallParentFunction)
  (Utilities|IsValid _returnvalue
    (:Is%20Valid
      (Input|AddMappingContext _returnvalue (Variables|Default|GetMappingContext) 0 "(bIgnoreAllPressedKeysUntilRelease=True,bForceImmediately=False,bNotifyUserSettings=False)"))))

(event EventTick
  (params (DeltaSeconds :type Float%20%28single-precision%29)))

(fn ConstructionScript)