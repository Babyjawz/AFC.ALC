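; Demo bow weapon Blueprint that manages the lifecycle of an arrow for a Character owner.
; MakeArrow spawns a BP_Demo_Arrow_AJ on the owner's hand mesh socket, then ConnectArrow and DisconnectArrow move it between that socket and the bow's skeletal mesh.
; FireArrow detaches and launches it, and DestroyArrow removes it.
; Connect, disconnect and fire also set the status on the CTCmptBowLite component.
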(event Custom|ConnectArrow
  (Default|SetBowStatus (Variables|Default|GetCT_Cmpt_Bow_Lite) "NewEnumerator0")
  (Utilities|FlowControl|Delay 0.1)
  (Transformation|AttachComponentToComponent (Variables|Default|GetArrowAJ) (Variables|Default|GetSkeletalMesh) "Arrow" "SnapToTarget" "SnapToTarget" "KeepRelative" true))

(event Custom|FireArrow
  (Default|SetBowStatus (Variables|Default|GetCT_Cmpt_Bow_Lite) "NewEnumerator2")
  (Transformation|DetachFromActor (Variables|Default|GetArrowAJ) "KeepWorld" "KeepWorld" "KeepWorld")
  (Default|Fire (Variables|Default|GetArrowAJ))
  (Variables|Default|SetArrowAJ 0))

(event Custom|MakeArrow
  (bind _returnvalue (Game|SpawnActorfromClass "/Game/BABYJAWS/Weapon/BP_Demo_Arrow_AJ.BP_Demo_Arrow_AJ_C" (Math|Transform|MakeTransform "0, 0, 0" "0, 0, 0" "1.000000,1.000000,1.000000") "Undefined" "MultiplyWithRoot" self 0))
  (Variables|Default|SetArrowAJ _returnvalue)
  (bind _ascharacter (Utilities|Casting|CastToCharacter (Components|GetOwner)))
  (Transformation|AttachComponentToComponent (Variables|Default|GetArrowAJ) (Variables|/Script/Engine.Character|GetMesh _ascharacter) "Arrow_Socket" "SnapToTarget" "SnapToTarget" "KeepRelative" true))

(event Custom|DisconnectArrow
  (bind _ascharacter (Utilities|Casting|CastToCharacter (Components|GetOwner)))
  (Transformation|AttachComponentToComponent (Variables|Default|GetArrowAJ) (Variables|/Script/Engine.Character|GetMesh _ascharacter) "Arrow_Socket" "SnapToTarget" "SnapToTarget" "KeepRelative" true)
  (Default|SetBowStatus (Variables|Default|GetCT_Cmpt_Bow_Lite) "NewEnumerator1"))

(event Custom|DestroyArrow
  (Actor|DestroyActor (Variables|Default|GetArrowAJ)))

(fn ConstructionScript)