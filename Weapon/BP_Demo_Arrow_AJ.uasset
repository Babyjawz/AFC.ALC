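; Demo arrow projectile that stays dormant until launched through ActivateFlight with a given velocity or through Fire.
; Fire launches along the actor's forward vector scaled by Distance, stores but does not aim at the hit point, clears lifespan and offsets the mesh after a brief delay.
; Both paths activate projectile movement and query-only sphere collision that ignores the owner and its owner while moving.
; No impact or damage logic is present.
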(event Custom|Activate%20Flight
  (params (Velocity :type Vector))
  (bind _projectilemovementcomp (Variables|Default|GetProjectileMovementComp))
  ;[0.9833 1 0.5] Activate Flight
  (Variables|/Script/Engine.MovementComponent|SetVelocity _projectilemovementcomp Velocity)
  (Components|Activation|Activate _projectilemovementcomp true)
  (CallFunction|ActivateCollision))

(event Custom|AdjustPosition
  (Utilities|FlowControl|Delay 0.01)
  (Transformation|SetRelativeLocation (Variables|Default|GetStaticMesh) (Math|Vector|MakeVector -4e+01 0.0 0.0) false false))

(event EventBeginPlay)

(event Collision|EventActorBeginOverlap
  (params (OtherActor :type Actor%20Object%20Reference)))

(event EventTick
  (params (DeltaSeconds :type Float%20%28single-precision%29)))

(fn ConstructionScript)

(fn ActivateCollision
  (bind _returnvalue (Components|GetOwner))
  (bind _spherecomp (Variables|Default|GetSphereComp))
  (Collision|IgnoreActorwhenMoving _spherecomp (Components|GetOwner _returnvalue) true)
  (Collision|IgnoreActorwhenMoving _spherecomp _returnvalue true)
  (Collision|SetCollisionEnabled _spherecomp "QueryOnly")
  (Collision|SetCollisionObjectType _spherecomp "ECC_GameTraceChannel1"))

(fn Fire
  (params (HitResult :type Hit%20Result%20Structure))
  (bind _projectilemovementcomp (Variables|Default|GetProjectileMovementComp))
  (Variables|Default|SetTargetLocation (.ImpactPoint (Collision|BreakHitResult HitResult)))
  (Variables|/Script/Engine.MovementComponent|SetVelocity _projectilemovementcomp (* (Transformation|GetActorForwardVector self) (Variables|Default|GetDistance)))
  (Components|Activation|Activate _projectilemovementcomp true)
  (CallFunction|ActivateCollision)
  (Actor|SetLifeSpan 0.0)
  (CallFunction|AdjustPosition))